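; Zombie enemy character that chases the player, attacks on arrival and dies when point damage depletes its health.
; An AI Move To loop targets the player controller, retrying on failure and playing an attack montage on success.
; When that montage completes, the chase restarts and the player pawn takes damage without a range check.
; Pawn sensing sets walk speed on sight; death stops movement, sets IsDead and plays a montage.
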(event `self.ReceiveBeginPlay`
  (`self.ChasePlayer`))

(event `ChasePlayer`
  (if (not (`self.IsDead`))
    ;[1 1 1] Chase Player Logic
    (`|AIMoveTo` self (0.0 0.0 0.0) (`GameplayStatics.GetPlayerController` 0) 100.0
      (:`OnSuccess`
        (`self.AttackPlayer`))
      (:`OnFail`
        (`self.ChasePlayer`)))))

(event `self.PawnSensing.OnSeePawn`
  (params (Pawn :type "Pawn Object Reference"))
  ;[1 1 1] Zombie Pawn Sensing
  (set `CharacterMovementComponent.MaxWalkSpeed` 360.0 (`self.CharacterMovement`)))

(event `AttackPlayer`
  ;[1 1 1] Attack Player
  (`|PlayMontage` (`self.Mesh`) "/Game/_Main/Characters/Zombie/Animation/zombie_attack_Montage.zombie_attack_Montage" 1.5
    (:`OnCompleted`
      (`self.ChasePlayer`)
      (`GameplayStatics.ApplyDamage` (`GameplayStatics.GetPlayerPawn` 0) 20.0))))

(event `self.ReceivePointDamage`
  (params (Damage :type "Float (single-precision)") (DamageType :type "DamageType Object Reference") (HitLocation :type "Vector Structure") (HitNormal :type "Vector Structure") (HitComponent :type "PrimitiveComponent Object Reference") (BoneName :type Name) (ShotFromDirection :type "Vector Structure") (InstigatedBy :type "Controller Object Reference") (DamageCauser :type "Actor Object Reference") (HitInfo :type "HitResult Structure (by ref)"))
  (if (not (`self.IsDead`))
    (set `self.Health` (- (`self.Health`) Damage))
    (if (<= (`self.Health`) 0.0)
      (`self.Death`))))

(event `Death`
  (set `self.IsDead` true)
  (`MovementComponent.StopMovementImmediately` (`self.CharacterMovement`))
  (`|PlayMontage` (`self.Mesh`) "/Game/_Main/Characters/Zombie/Animation/zombie_death_Montage.zombie_death_Montage"))

(fn `UserConstructionScript`)