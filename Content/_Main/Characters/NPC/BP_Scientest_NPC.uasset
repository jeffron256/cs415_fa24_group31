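; Scientist NPC Blueprint that shows its dialog one line at a time through a Talk event.
; Each Talk call advances TalkIndex, prints that DialogContent entry and shows it in a WB_Dialog widget, created when no valid one exists.
; Once the index passes the last entry, it removes the widget and sets a finished flag, with no reset to replay the dialog.
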(event `/Game/_Main/Characters/NPC/BPI_NPC_Dialog.Talk`
  (bind _talkindex (`self.TalkIndex`))
  (bind _dialogcontent (`self.DialogContent`))
  (`/Engine/EditorBlueprintResources/StandardMacros.IncrementInt` _talkindex
    (:`  `
      (if (< _talkindex (`KismetArrayLibrary.Array_Length` _dialogcontent))
        (`KismetSystemLibrary.PrintString` (`|GetArrayItem` _dialogcontent (`self.TalkIndex`)))
        (`self.UI`
          (:`then`
            _)
          (:`else`
            (bind _returnvalue (`|CreateWidget` "/Game/_Main/Characters/NPC/WB_Dialog.WB_Dialog_C" (`GameplayStatics.GetPlayerController` 0)))
            (bind _output_get (set `self.UI` _returnvalue))
            (`UserWidget.AddToViewport` _output_get 0)))
        (`TextBlock.SetText` (`/Game/_Main/Characters/NPC/WB_Dialog.DialogContent` (`self.UI`)) (`KismetTextLibrary.Conv_StringToText` (`|GetArrayItem` (`self.DialogContent`) (`self.TalkIndex`))))
        (elif (!= (`self.Dialog FInished`) true)
          (`Widget.RemoveFromParent` (`self.UI`))
          (set `self.Dialog FInished` true))))))

(fn `UserConstructionScript`)